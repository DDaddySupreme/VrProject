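; A VR gun actor that a motion controller can pick up and drop, toggling physics as it attaches or detaches.
; FireWeapon spends a round, updates the ammo text, plays sound and muzzle flash, and spawns a bullet.
; A timeline then animates the bolt and, on an event track, ejects a shell with smoke.
; Overlapping an Ammo actor with the fill volume adds its quantity, clamped to the maximum, and destroys it.
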(event `self.ReceiveBeginPlay`
  (`TextRenderComponent.K2_SetText` (`self.TextRender`) (`KismetTextLibrary.Conv_IntToText` (`self.AmmoAmount`))))

(event `self.AmmoFill.OnComponentBeginOverlap`
  (params (OverlappedComponent :type "PrimitiveComponent Object Reference") (OtherActor :type "Actor Object Reference") (OtherComp :type "PrimitiveComponent Object Reference") (OtherBodyIndex :type Integer) (bFromSweep :type Boolean) (SweepResult :type "HitResult Structure (by ref)"))
  (bind _asammo (cast `/Game/Blueprints/Ammo` OtherActor))
  (`/Game/VirtualRealityBP/Blueprints/PickupActorInterface.Drop` _asammo)
  (`KismetSystemLibrary.PrintString` "Ammo Detected")
  (bind _output_get (set `self.AmmoAmount` (`KismetMathLibrary.Clamp` (+ (`self.AmmoAmount`) (`/Game/Blueprints/Ammo.Quantity` _asammo)) 0 (`self.MaxAmmo`))))
  (`TextRenderComponent.K2_SetText` (`self.TextRender`) (`KismetTextLibrary.Conv_IntToText` _output_get))
  (`/Game/Blueprints/Ammo.Drop` _asammo)
  (`self.K2_DestroyActor` _asammo))

(event `/Game/VirtualRealityBP/Blueprints/PickupActorInterface.Pickup`
  (params (AttachTo :type "SceneComponent Object Reference"))
  (`PrimitiveComponent.SetSimulatePhysics` (`self.StaticMesh`) false)
  (`SceneComponent.K2_AttachToComponent` (`self.K2_GetRootComponent`) AttachTo "None" "KeepWorld" "KeepWorld" "KeepWorld" false))

(event `/Game/VirtualRealityBP/Blueprints/PickupActorInterface.Drop`
  (`PrimitiveComponent.SetSimulatePhysics` (`self.StaticMesh`) true)
  (`self.K2_DetachFromActor` "KeepWorld" "KeepWorld" "KeepWorld"))

(event `FireWeapon`
  (if (> (`self.AmmoAmount`) 0)
    (bind _output_get (set `self.AmmoAmount` (- (`self.AmmoAmount`) 1)))
    (`TextRenderComponent.K2_SetText` (`self.TextRender`) (`KismetTextLibrary.Conv_IntToText` _output_get))
    (`|ExecutionSequence`
      (:`then_0`
        (`GameplayStatics.PlaySoundAtLocation` "/Game/StarterContent/Audio/Explosion01.Explosion01" (`SceneComponent.K2_GetComponentLocation` (`self.Shell`)) (struct) 2.0))
      (:`then_1`
        (`ActorComponent.Activate` (`self.MuzzleFlash`) true))
      (:`then_2`
        (`|SpawnActorFromClass` "/Game/Blueprints/Bullet.Bullet_C" (`SceneComponent.K2_GetComponentToWorld` (`self.Scene`)) "AlwaysSpawn" "OverrideRootScale" self (`GameplayStatics.GetPlayerPawn` 0))
        (bind (_direction _lerp) (`Timeline|BoltAction` :!via `PlayFromStart`)
          (:`Update`
            (`SceneComponent.K2_SetRelativeTransform` (`self.Bolt`) (`KismetMathLibrary.TLerp` (`KismetMathLibrary.MakeTransform` (0.0 0.0 0.0)) (`KismetMathLibrary.MakeTransform` (-490.0 0.0 0.0)) _lerp) false false))
          (:`LaunchShell`
            (`|SpawnActorFromClass` "/Game/Blueprints/Shell.Shell_C" (`SceneComponent.K2_GetComponentToWorld` (`self.Shell`)) "AlwaysSpawn" "OverrideRootScale" null null)
            (`ActorComponent.Activate` (`self.Bolt Smoke`) true)))))
    (else
      (`KismetSystemLibrary.PrintString` "Out of Ammo"))))

(fn `UserConstructionScript`)